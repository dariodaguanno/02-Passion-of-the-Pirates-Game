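; Possessable cannon pawn that the player enters to aim and fire projectiles, with a predicted trajectory as a pointer.
; Interact hides the interactor and possesses the cannon; the Interact input restores it at the cannon mesh and returns possession.
; Mouse axes yaw the cart and tilt the clamped barrel, while left click plays a sound and spawns a projectile.
; Tick debug-draws the predicted path from the muzzle socket, and box overlaps toggle a prompt marker for the third-person character.
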(event `/Game/Cannon/Blueprints/InteractInterface_BI.Interact`
  (params (Interactor :type "/Game/ThirdPersonBP/Blueprints/ThirdPersonCharacter Object Reference"))
  ;[1 1 1] enter to " Cannon "  -  press "e"
  (`self.SetActorHiddenInGame` Interactor true)
  (`self.SetActorEnableCollision` Interactor false)
  (`Controller.Possess` (`GameplayStatics.GetPlayerController` 0) self))

(event `InputAction|Interact`
  (params (Key :type "Key Structure"))
  ;[1 1 1] enter to " Cannon "  -  press "e"
  (:`Pressed`
    (`self.K2_SetActorLocation` (stale `/Game/Cannon/Blueprints/InteractInterface_BI.Interact` Interactor) (`SceneComponent.K2_GetComponentLocation` (`self.SkeletalMesh`)) false false)
    (`self.SetActorHiddenInGame` (stale `/Game/Cannon/Blueprints/InteractInterface_BI.Interact` Interactor) false)
    (`self.SetActorEnableCollision` (stale `/Game/Cannon/Blueprints/InteractInterface_BI.Interact` Interactor) true)
    (`Controller.Possess` (`GameplayStatics.GetPlayerController` 0) (stale `/Game/Cannon/Blueprints/InteractInterface_BI.Interact` Interactor))))

(event `InputAxis|LookUp`
  (params (AxisValue :type "Float (single-precision)"))
  ;[1 1 1] MOVE SHOOT Above And Under
  (set `self.Connon Rot Pitch` (`KismetMathLibrary.FClamp` (+ (`self.Connon Rot Pitch`) AxisValue) -50.0 100.0))
  (`SceneComponent.K2_SetRelativeRotation` (`self.The_barrel_of_the_cannon_StaticMesh_2`) (`KismetMathLibrary.MakeRotator` (`self.Connon Rot Pitch`) (.yaw (`SceneComponent.RelativeRotation` (`self.The_barrel_of_the_cannon_StaticMesh_2`))) (.pitch (`SceneComponent.RelativeRotation` (`self.The_barrel_of_the_cannon_StaticMesh_2`)))) false false))

(event `Key|LeftMouseButton`
  (params (Key :type "Key Structure"))
  ;[1 0.1643 0.3042] SHOOT FIRE
  (:`Pressed`
    (`GameplayStatics.PlaySound2D` null 1.0 1.0 0.0 null null)
    (`self.Shoot`)))

(event `self.ReceiveTick`
  (params (DeltaSeconds :type "Float (single-precision)"))
  (bind (_returnvalue_location _returnvalue_rotation) (`KismetMathLibrary.BreakTransform` (`SceneComponent.GetSocketTransform` (`self.Shoot_Zone`) "AmmoEject" "RTS_World")))
  (bind _returnvalue (`KismetMathLibrary.GetForwardVector` _returnvalue_rotation))
  ;[0.06569 1 0.07899] select SHOOT ARRAY LINE
  (`GameplayStatics.Blueprint_PredictProjectilePath_ByObjectType` :`StartPos` _returnvalue_location :`LaunchVelocity` (* (+ _returnvalue (* _returnvalue (`self.Direction`))) (`self.Speed`)) :`ProjectileRadius` 20.0 :`ObjectTypes` (`|MakeArray` "ObjectTypeQuery1" :!type "EObjectTypeQuery Enum") :`DrawDebugType` "ForDuration" :`MaxSimTime` 10.0))

(event `Shoot`
  (bind _shoot_zone (`self.Shoot_Zone`))
  ;[1 0.1643 0.3042] SHOOT FIRE
  (`|SpawnActorFromClass` "/Game/Cannon/Blueprints/Projectile_Base_Child_BP.Projectile_Base_Child_BP_C" (`KismetMathLibrary.MakeTransform` (`SceneComponent.K2_GetComponentLocation` _shoot_zone) (`SceneComponent.K2_GetComponentRotation` _shoot_zone)) "Undefined" "OverrideRootScale" null null))

(event `self. Box.OnComponentBeginOverlap`
  (params (OverlappedComponent :type "PrimitiveComponent Object Reference") (OtherActor :type "Actor Object Reference") (OtherComp :type "PrimitiveComponent Object Reference") (OtherBodyIndex :type Integer) (bFromSweep :type Boolean) (SweepResult :type "HitResult Structure (by ref)"))
  ;[1 0.4258 0.4059] Show control buttons - Press ''E'' Button
  (cast `/Game/ThirdPersonBP/Blueprints/ThirdPersonCharacter` OtherActor)
  (`SceneComponent.ToggleVisibility` (`self.WorldMarker4`) true))

(event `InputAxis|Rotate the mouse`
  (params (AxisValue :type "Float (single-precision)"))
  (bind _cannon_cart_staticmesh_1 (`self.Cannon_cart_StaticMesh_1`))
  (bind (_returnvalue_roll _returnvalue_pitch _returnvalue_yaw) (`KismetMathLibrary.BreakRotator` (`SceneComponent.K2_GetComponentRotation` _cannon_cart_staticmesh_1)))
  ;[0.4775 0.7954 1] MOVE SHOOT RIGHT /LEFT
  (bind _output_get (set `self.TargetRotation` (`KismetMathLibrary.MakeRotator` _returnvalue_roll _returnvalue_pitch (+ AxisValue _returnvalue_yaw))))
  (`SceneComponent.K2_SetRelativeRotation` _cannon_cart_staticmesh_1 _output_get false false))

(event `self. Box.OnComponentEndOverlap`
  (params (OverlappedComponent :type "PrimitiveComponent Object Reference") (OtherActor :type "Actor Object Reference") (OtherComp :type "PrimitiveComponent Object Reference") (OtherBodyIndex :type Integer))
  ;[1 0.4258 0.4059] Show control buttons - Press ''E'' Button
  (cast `/Game/ThirdPersonBP/Blueprints/ThirdPersonCharacter` OtherActor)
  (`SceneComponent.ToggleVisibility` (`self.WorldMarker4`) true))

(fn `UserConstructionScript`)
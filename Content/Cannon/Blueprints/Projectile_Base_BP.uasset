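; Base cannon projectile that handles impact feedback and optional explosive area damage when its Hit event fires.
; On hit it swaps the particle template, plays a sound, disables sphere collision and destroys itself after a short delay.
; If Explosion is set, it sends overlapped Pawns a DamageMessage with linear distance falloff and an unscaled outward impulse on the pelvis.
; The non-explosive branch only prints a debug string.
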(event `self.ReceiveHit`
  (params (MyComp :type "PrimitiveComponent Object Reference") (Other :type "Actor Object Reference") (OtherComp :type "PrimitiveComponent Object Reference") (bSelfMoved :type Boolean) (HitLocation :type "Vector Structure") (HitNormal :type "Vector Structure") (NormalImpulse :type "Vector Structure") (Hit :type "HitResult Structure (by ref)"))
  (bind _hit_location (`self.Hit Location`))
  (set `self.Hit Location` HitLocation)
  (`|ExecutionSequence`
    (:`then_0`
      (`ParticleSystemComponent.SetTemplate` (`self.ParticleSystem`) (`self.HitEffect`))
      (`GameplayStatics.PlaySoundAtLocation` (`self.HitSound`) (`self.K2_GetActorLocation`) (struct) 1.0 1.0 0.0 null null null)
      (`PrimitiveComponent.SetCollisionEnabled` (`self.Sphere`) "NoCollision")
      (`KismetSystemLibrary.Delay` 1.5)
      (`self.K2_DestroyActor`))
    (:`then_1`
      (if (`self.Explosion`)
        (bind _outactors (`KismetSystemLibrary.SphereOverlapActors` (`self.Hit Location`) (`self.ExplosionRadius`) (`|MakeArray` "ObjectTypeQuery3" :!type "EObjectTypeQuery Enum")))
        (for _array_element _outactors
          (bind _returnvalue (`self.K2_GetActorLocation` _array_element))
          (message `/Game/Cannon/Blueprints/Damage_Interface_BI.Damage` _array_element (* (`KismetMathLibrary.FClamp` (- 1.0 (/ (`KismetMathLibrary.VSize` (- _returnvalue (`self.Hit Location`))) (`self.ExplosionRadius`)))) (`self.DamagePercent`)) "NewEnumerator0" "Pelvis" (* (`KismetMathLibrary.GetDirectionUnitVector` _hit_location _returnvalue) (`self.Impules`)) _hit_location))
        (else
          (`KismetSystemLibrary.PrintString` "Hello"))))))

(fn `UserConstructionScript`)
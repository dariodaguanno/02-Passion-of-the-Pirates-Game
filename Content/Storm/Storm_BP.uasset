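; Storm is a battle-royale-style shrinking zone actor that damages the player outside its bounds.
; A Shrink timeline starts shortly after BeginPlay and drives the static mesh's world scale.
; Any actor ending overlap sets InStorm and starts a delay loop calling TakeDamage5 on player 0's ThirdPersonCharacter every half second.
; Any actor beginning overlap clears InStorm to end the loop, without checking which actor overlapped.
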(event `self.ReceiveBeginPlay`
  (`KismetSystemLibrary.Delay` 0.2)
  (bind (_direction _shrink_track) (`Timeline|Shrink`)
    (:`Update`
      (`SceneComponent.SetWorldScale3D` (`self.StaticMesh`) (`KismetMathLibrary.Conv_DoubleToVector` _shrink_track)))))

(event `self.StaticMesh.OnComponentBeginOverlap`
  (params (OverlappedComponent :type "PrimitiveComponent Object Reference") (OtherActor :type "Actor Object Reference") (OtherComp :type "PrimitiveComponent Object Reference") (OtherBodyIndex :type Integer) (bFromSweep :type Boolean) (SweepResult :type "HitResult Structure (by ref)"))
  ;[1 1 1] Player in/out of Storm
)

(event `self.ReceiveActorEndOverlap`
  (params (OtherActor :type "Actor Object Reference"))
  ;[1 1 1] Player in/out of Storm
  (bind _asthird_person_character (cast `/Game/ThirdPersonBP/Blueprints/ThirdPersonCharacter` (`GameplayStatics.GetPlayerCharacter` 0)))
  (set `self.InStorm` true)
  (`/Game/ThirdPersonBP/Blueprints/ThirdPersonCharacter.TakeDamage5%` _asthird_person_character :!label _label)
  (if (`self.InStorm`)
    (`KismetSystemLibrary.Delay` 0.5)
    (goto _label)))

(event `self.StaticMesh.OnComponentEndOverlap`
  (params (OverlappedComponent :type "PrimitiveComponent Object Reference") (OtherActor :type "Actor Object Reference") (OtherComp :type "PrimitiveComponent Object Reference") (OtherBodyIndex :type Integer))
  ;[1 1 1] Player in/out of Storm
)

(event `self.ReceiveActorBeginOverlap`
  (params (OtherActor :type "Actor Object Reference"))
  ;[1 1 1] Player in/out of Storm
  (set `self.InStorm` false))

(fn `UserConstructionScript`)
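; Cannon Blueprint that automatically fires projectiles while a SimpleAI actor is in range.
; Overlap begin and end events on the Range component set and clear a single Active flag, without counting how many AI are inside.
; Tick gates firing through a short Delay, so FireCannon repeats at intervals, playing a 2D sound and spawning a Cannon_projectile at a rotated offset from Sphere, aligned to the Scene component's rotation.
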(event `self.ReceiveTick`
  (params (DeltaSeconds :type "Float (single-precision)"))
  (if (`self.active`)
    (`KismetSystemLibrary.Delay` 0.1)
    (`self.FireCannon`)))

(event `self.range.OnComponentBeginOverlap`
  (params (OverlappedComponent :type "PrimitiveComponent Object Reference") (OtherActor :type "Actor Object Reference") (OtherComp :type "PrimitiveComponent Object Reference") (OtherBodyIndex :type Integer) (bFromSweep :type Boolean) (SweepResult :type "HitResult Structure (by ref)"))
  (cast `/Game/ThirdPersonBP/Blueprints/SimpleAI` OtherActor)
  (set `self.active` true))

(event `self.range.OnComponentEndOverlap`
  (params (OverlappedComponent :type "PrimitiveComponent Object Reference") (OtherActor :type "Actor Object Reference") (OtherComp :type "PrimitiveComponent Object Reference") (OtherBodyIndex :type Integer))
  (cast `/Game/ThirdPersonBP/Blueprints/SimpleAI` OtherActor)
  (set `self.active` false))

(event `FireCannon`
  (bind _returnvalue (`SceneComponent.K2_GetComponentRotation` (`self.Scene`)))
  (`GameplayStatics.PlaySound2D` "/Game/StarterContent/Audio/Collapse01.Collapse01" 1.0 1.0 0.0 null null)
  (`|SpawnActorFromClass` "/Game/Cannon/cannon_projectile.cannon_projectile_C" (`KismetMathLibrary.MakeTransform` (+ (`SceneComponent.K2_GetComponentLocation` (`self.Sphere`)) (`KismetMathLibrary.GreaterGreater_VectorRotator` (`self.offset`) _returnvalue)) _returnvalue) "Undefined" "OverrideRootScale" null null))

(fn `UserConstructionScript`)